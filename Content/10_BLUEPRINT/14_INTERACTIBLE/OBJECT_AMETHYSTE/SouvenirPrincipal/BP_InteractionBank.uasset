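; BP_InteractionBank holds three choice interactions (A, B, C), apparently for the main memory ("SouvenirPrincipal") interactible.
; Each event creates a player for the level sequence in its matching LevelSequence variable and starts playback.
; It then immediately passes that variable's next choice and appearance delay to BM.NextChoice, never flagging the end, so choices chain through data.
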(event `/Game/10_BLUEPRINT/14_INTERACTIBLE/OBJECT_AMETHYSTE/BP_ParentObject.InteractionA`
  (params (Player :type "/Game/10_BLUEPRINT/12_CONTROLLER/BP_CHARACTER Object Reference"))
  (bind (_levelsequencea_animtoplay _levelsequencea_nextchoice _levelsequencea_delay) (break `/Game/10_BLUEPRINT/18_PARAMETERS/STRUCTURE/Cinematique` (`self.LevelSequenceA`)))
  (bind (_outactor _returnvalue) (`LevelSequencePlayer.CreateLevelSequencePlayer` _levelsequencea_animtoplay))
  (`MovieSceneSequencePlayer.Play` _returnvalue)
  (`/Game/10_BLUEPRINT/14_INTERACTIBLE/OBJECT_AMETHYSTE/SouvenirPrincipal/BP_BanqueManager.NextChoice` (`self.BM`) _levelsequencea_nextchoice _levelsequencea_delay false))

(event `/Game/10_BLUEPRINT/14_INTERACTIBLE/OBJECT_AMETHYSTE/BP_ParentObject.InteractionB`
  (params (Player :type "/Game/10_BLUEPRINT/12_CONTROLLER/BP_CHARACTER Object Reference"))
  (bind (_levelsequenceb_animtoplay _levelsequenceb_nextchoice _levelsequenceb_delay) (break `/Game/10_BLUEPRINT/18_PARAMETERS/STRUCTURE/Cinematique` (`self.LevelSequenceB`)))
  (bind (_outactor _returnvalue) (`LevelSequencePlayer.CreateLevelSequencePlayer` _levelsequenceb_animtoplay))
  (`MovieSceneSequencePlayer.Play` _returnvalue)
  (`/Game/10_BLUEPRINT/14_INTERACTIBLE/OBJECT_AMETHYSTE/SouvenirPrincipal/BP_BanqueManager.NextChoice` (`self.BM`) _levelsequenceb_nextchoice _levelsequenceb_delay false))

(event `/Game/10_BLUEPRINT/14_INTERACTIBLE/OBJECT_AMETHYSTE/BP_ParentObject.InteractionC`
  (params (Player :type "/Game/10_BLUEPRINT/12_CONTROLLER/BP_CHARACTER Object Reference"))
  (bind (_levelsequencec_animtoplay _levelsequencec_nextchoice _levelsequencec_delay) (break `/Game/10_BLUEPRINT/18_PARAMETERS/STRUCTURE/Cinematique` (`self.LevelSequenceC`)))
  (bind (_outactor _returnvalue) (`LevelSequencePlayer.CreateLevelSequencePlayer` _levelsequencec_animtoplay))
  (`MovieSceneSequencePlayer.Play` _returnvalue)
  (`/Game/10_BLUEPRINT/14_INTERACTIBLE/OBJECT_AMETHYSTE/SouvenirPrincipal/BP_BanqueManager.NextChoice` (`self.BM`) _levelsequencec_nextchoice _levelsequencec_delay false))

(fn `UserConstructionScript`
  (`parent.UserConstructionScript`))