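; BP_BanqueManager is a manager actor that controls which set of choice actors in its Choice array is visible and interactible.
; On BeginPlay it reveals the initial set and enables query-only collision on each actor's Cylinder.
; NextChoice hides and disables the current set, waits a given delay, then stores and reveals the new set with query and physics collision.
; When NextChoice receives End as true, it leaves everything unchanged.
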(event `self.ReceiveBeginPlay`
  (`self.StartBank`))

(event `StartBank`
  (for _array_element (`self.Choice`)
    (`self.SetActorHiddenInGame` _array_element false)
    (`PrimitiveComponent.SetCollisionEnabled` (`/Game/10_BLUEPRINT/14_INTERACTIBLE/OBJECT_AMETHYSTE/SouvenirPrincipal/BP_BanqueTest.Cylinder` _array_element) "QueryOnly")))

(event `NextChoice`
  (params (NewChoice :type "Array of /Game/10_BLUEPRINT/14_INTERACTIBLE/OBJECT_AMETHYSTE/SouvenirPrincipal/BP_InteractionBank Object Reference") (ApparitionDelay :type "Float (double-precision)") (End :type Boolean))
  (if (not End)
    (set `self.NewChoice` NewChoice)
    (for _array_element (`self.Choice`)
      (`self.SetActorHiddenInGame` _array_element true)
      (`PrimitiveComponent.SetCollisionEnabled` (`/Game/10_BLUEPRINT/14_INTERACTIBLE/OBJECT_AMETHYSTE/SouvenirPrincipal/BP_BanqueTest.Cylinder` _array_element) "NoCollision"))
    (`KismetSystemLibrary.Delay` ApparitionDelay)
    (bind _output_get (set `self.Choice` (`self.NewChoice`)))
    (for _array_element_2 _output_get
      (`self.SetActorHiddenInGame` _array_element_2 false)
      (`PrimitiveComponent.SetCollisionEnabled` (`/Game/10_BLUEPRINT/14_INTERACTIBLE/OBJECT_AMETHYSTE/SouvenirPrincipal/BP_BanqueTest.Cylinder` _array_element_2) "QueryAndPhysics"))))

(fn `UserConstructionScript`)