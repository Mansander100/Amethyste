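; Interactible object the player can inspect up close or carry with a physics handle, child of a parent interactible Blueprint.
; InteractionA toggles inspection: a reversible Zoom timeline moves the mesh to the player's arrow while movement and look are locked, and Inspect rotates it relative to camera yaw.
; InteractionB toggles grabbing, snapping on release.
; Grabbing runs optionally one-shot actions (only Dialogue is functional) and notifies the ReminiscenceManager.
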(event `Inspect`
  (params (X :type "Float (double-precision)") (Y :type "Float (double-precision)") (Player :type "/Game/10_BLUEPRINT/12_CONTROLLER/BP_CHARACTER Object Reference"))
  (bind (_returnvalue_roll _returnvalue_pitch _returnvalue_yaw) (`KismetMathLibrary.BreakRotator` (`SceneComponent.K2_GetComponentRotation` (`/Game/10_BLUEPRINT/12_CONTROLLER/BP_CHARACTER.CineCamera` Player))))
  (`SceneComponent.K2_AddWorldRotation` (`self.Mesh`) (* (`KismetMathLibrary.Conv_VectorToRotator` (`KismetMathLibrary.GreaterGreater_VectorRotator` (`KismetMathLibrary.MakeVector` 0.0 (* X -1.0) (* Y 1.0)) (`KismetMathLibrary.MakeRotator` 0.0 0.0 _returnvalue_yaw))) (`self.Speed`)) false false))

(event `self.InteractionA`
  (params (Player :type "/Game/10_BLUEPRINT/12_CONTROLLER/BP_CHARACTER Object Reference"))
  (bind _output_get (set `self.Player` Player))
  ;[1 1 1] verifie si on est deja entrain d'inspecter
  (if (not (`self.isInspecting`))
    (set `self.StartPoint` (`SceneComponent.K2_GetComponentToWorld` (`self.Mesh`)))
    (set `self.EndPoint` (`SceneComponent.K2_GetComponentToWorld` (`/Game/10_BLUEPRINT/12_CONTROLLER/BP_CHARACTER.Arrow1` _output_get)))
    (`PrimitiveComponent.SetEnableGravity` (`self.Mesh`) false)
    (set `/Game/10_BLUEPRINT/12_CONTROLLER/BP_CHARACTER.canMove` false _output_get)
    (set `/Game/10_BLUEPRINT/12_CONTROLLER/BP_CHARACTER.canLook` false _output_get)
    (set `self.isInspecting` true)
    (set `/Game/10_BLUEPRINT/12_CONTROLLER/BP_CHARACTER.IsInspectingObject` true _output_get)
    (`PrimitiveComponent.SetCollisionEnabled` (`self.Mesh`) "QueryOnly")
    (bind (_direction _delta) (`Timeline|zoom` :!label _label)
      (:`Update`
        (`SceneComponent.K2_SetWorldTransform` (`self.Mesh`) (`KismetMathLibrary.MakeTransform` (.location (`KismetMathLibrary.TLerp` (`self.StartPoint`) (`self.EndPoint`) _delta)) (.rotation (`KismetMathLibrary.TLerp` (`self.StartPoint`) (`self.EndPoint`) _delta)) (`SceneComponent.RelativeScale3D` (`self.Mesh`))) false false))
      (:`Finished`
        (if (not (`self.isInspecting`))
          (`PrimitiveComponent.SetCollisionEnabled` (`self.Mesh`) "QueryAndPhysics")
          (`PrimitiveComponent.SetEnableGravity` (`self.Mesh`) true))))
    (else
      (set `/Game/10_BLUEPRINT/12_CONTROLLER/BP_CHARACTER.canMove` true _output_get)
      (set `/Game/10_BLUEPRINT/12_CONTROLLER/BP_CHARACTER.canLook` true _output_get)
      (set `self.isInspecting` false)
      (set `/Game/10_BLUEPRINT/12_CONTROLLER/BP_CHARACTER.IsInspectingObject` false _output_get)
      (goto _label :!via `Reverse`))))

(event `self.InteractionB`
  (params (Player :type "/Game/10_BLUEPRINT/12_CONTROLLER/BP_CHARACTER Object Reference"))
  (bind _reminiscencemanager (`self.ReminiscenceManager`))
  (bind _snap (`self.Snap`))
  ;[0.02604 0.02604 0.02604] Grab Object
  (bind _output_get (set `self.Player` Player))
  (if (`/Game/10_BLUEPRINT/12_CONTROLLER/BP_CHARACTER.IsGrabbingObject` _output_get)
    (bind _physicshandle (`/Game/10_BLUEPRINT/12_CONTROLLER/BP_CHARACTER.PhysicsHandle` _output_get))
    (`PhysicsHandleComponent.ReleaseComponent` _physicshandle)
    (set `/Game/10_BLUEPRINT/12_CONTROLLER/BP_CHARACTER.IsGrabbingObject` false _output_get)
    (`SceneComponent.SetVisibility` (`/Game/10_BLUEPRINT/12_CONTROLLER/BP_CHARACTER.Decal` _output_get) false false)
    (`/Engine/EditorBlueprintResources/StandardMacros.IsValid` _snap
      (:`Is Valid`
        (`/Game/10_BLUEPRINT/13_GAS/Trigger/BP_CollectZoneSnap_AND.Snap` _snap self)))
    (else
      (set `/Game/10_BLUEPRINT/12_CONTROLLER/BP_CHARACTER.IsGrabbingObject` true _output_get)
      (bind _returnvalue (`self.GetComponentByClass` (`/Game/10_BLUEPRINT/12_CONTROLLER/BP_CHARACTER.InteractibleObject` _output_get) "/Script/Engine.PrimitiveComponent"))
      (`PhysicsHandleComponent.GrabComponentAtLocationWithRotation` :`self` _physicshandle :`Component` _returnvalue :`Location` (`SceneComponent.K2_GetComponentLocation` _returnvalue))
      (`self.IsLooked` false)
      (`SceneComponent.SetVisibility` (`/Game/10_BLUEPRINT/12_CONTROLLER/BP_CHARACTER.Decal` _output_get) true false)
      (`self.DoGrabAction`)
      (`/Engine/EditorBlueprintResources/StandardMacros.IsValid` _reminiscencemanager
        (:`Is Valid`
          (`/Game/10_BLUEPRINT/15_MANAGER/BP_ReminiscenceManager.CheckRightAction?` _reminiscencemanager self))))))

(fn `DoGrabAction`
  (for _array_element (`self.Action`)
    (bind (_action _doonce _indexdialogue _timedialogue) (break `/Game/10_BLUEPRINT/18_PARAMETERS/STRUCTURE/ActionGrab` _array_element))
    (if (not _doonce)
      (switch `/Game/10_BLUEPRINT/18_PARAMETERS/ENUMERATION/ActionType` (`.type_9_2EBDAB05448CCA25048AAF98040B5719` (break `/Game/10_BLUEPRINT/18_PARAMETERS/STRUCTURE/ActionType` _action)) :!label _label
        (:`NewEnumerator0`
          (`KismetSystemLibrary.PrintString` "1"))
        (:`NewEnumerator1`
          (`KismetSystemLibrary.PrintString` "2"))
        (:`NewEnumerator2`
          (`KismetSystemLibrary.PrintString` "3"))
        (:`NewEnumerator3`
          (`/Game/10_BLUEPRINT/15_MANAGER/BP_GeneralManager.ShowDialogue` (`/Game/10_BLUEPRINT/15_MANAGER/BP_ReminiscenceManager.GeneralManager` (`self.ReminiscenceManager`)) _indexdialogue _timedialogue)
          (`KismetSystemLibrary.PrintString` "4")))
      (elif (not (`self.Already grabed`))
        (goto _label))))
  (set `self.Already grabed` true))

(fn `Return To Base`
  (bind _mesh (`self.Mesh`))
  (`SceneComponent.K2_SetRelativeLocation` _mesh (`SceneComponent.RelativeLocation` (`self.DefaultSceneRoot`)) false false)
  (`PrimitiveComponent.SetPhysicsLinearVelocity` _mesh (0.0 0.0 0.0) false "None")
  (`/Game/10_BLUEPRINT/12_CONTROLLER/BP_CHARACTER.ReleaseObject` (`self.Player`)))

(fn `UserConstructionScript`
  (`parent.UserConstructionScript`))