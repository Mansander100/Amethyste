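; Interactive furniture door that swings open and closed when the player triggers InteractionB.
; BeginPlay stores the mesh's relative rotation, and a FlipFlop alternately plays and reverses a Timeline that lerps from that rotation to the target.
; The target comes from an X-axis direction vector built with negated AngleOuverture on Y, so only that value's sign affects the absolute relative rotation reached, not its magnitude.
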(event `self.ReceiveBeginPlay`
  (set `self.StartRot` (`SceneComponent.RelativeRotation` (`self.Mesh`))))

(event `self.InteractionB`
  (params (Player :type "/Game/10_BLUEPRINT/12_CONTROLLER/BP_CHARACTER Object Reference"))
  (`/Engine/EditorBlueprintResources/StandardMacros.FlipFlop`
    (:`A`
      (bind (_direction _delta) (`Timeline|Timeline` :!label _label)
        (:`Update`
          (`SceneComponent.K2_SetRelativeRotation` (`self.Mesh`) (`KismetMathLibrary.RLerp` (`self.StartRot`) (`KismetMathLibrary.Conv_VectorToRotator` (`KismetMathLibrary.MakeVector` 0.0 (* (`self.AngleOuverture`) -1.0))) _delta) false false))))
    (:`B`
      (goto _label :!via `Reverse`))))

(fn `UserConstructionScript`
  (`parent.UserConstructionScript`))