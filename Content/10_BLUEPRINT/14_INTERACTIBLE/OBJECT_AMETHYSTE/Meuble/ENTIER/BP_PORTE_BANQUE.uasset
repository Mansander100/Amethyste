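; BP_PORTE_BANQUE is an interactable double bank door that opens only when CanOpen is set.
; InteractionB passes through a DoOnce to OpenDoor, which plays or reverses a Timeline based on Open, swinging both meshes in opposite yaw directions.
; When locked, it shows a dialogue through GeneralManager and calls ResetDoor to re-arm the DoOnce.
; The successful branch never resets that gate itself.
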(event `OpenDoor`
  (if (`self.CanOpen`)
    (if (`self.Open?`)
      (set `self.Open?` false)
      (bind (_direction _newtrack_0) (`Timeline|Timeline` :!label _label)
        (:`Update`
          (`SceneComponent.K2_SetRelativeRotation` (`self.Mesh`) (`KismetMathLibrary.MakeRotator` 0.0 0.0 (`KismetMathLibrary.Lerp` 90.0 200.0 _newtrack_0)) false false)
          (`SceneComponent.K2_SetRelativeRotation` (`self.Mesh1`) (`KismetMathLibrary.MakeRotator` 0.0 0.0 (`KismetMathLibrary.Lerp` 90.0 -20.0 _newtrack_0)) false false)))
      (else
        (set `self.Open?` true)
        (goto _label :!via `Reverse`)))
    (else
      (`/Game/10_BLUEPRINT/15_MANAGER/BP_GeneralManager.ShowDialogue` :`self` (`self.generalManager`) :`index` 15 :`Duration` 5.0)
      (`self.ResetDoor`))))

(event `self.InteractionB`
  (params (Player :type "/Game/10_BLUEPRINT/12_CONTROLLER/BP_CHARACTER Object Reference"))
  (`/Engine/EditorBlueprintResources/StandardMacros.DoOnce` false :!label _label_2
    (:`Completed`
      (`self.OpenDoor`))))

(event `ResetDoor`
  (goto _label_2 :!via `Reset`))

(fn `UserConstructionScript`
  (`parent.UserConstructionScript`))