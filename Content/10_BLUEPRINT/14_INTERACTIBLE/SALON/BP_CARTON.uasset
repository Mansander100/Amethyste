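; BP_CARTON is an interactable cardboard box in the salon that reacts once when used.
; InteractionA, gated by a DoOnce, plays a timeline that incrementally rotates Cube1 in yaw through a lerp on the Delta track.
; The timeline update also unhides the TRIGGER actors, shows Text, then shows the TextNext entries after a delay.
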(event `self.InteractionA`
  (params (Player :type "/Game/10_BLUEPRINT/12_CONTROLLER/BP_CHARACTER Object Reference"))
  (`/Engine/EditorBlueprintResources/StandardMacros.DoOnce` false
    (:`Completed`
      (bind (_direction _delta) (`Timeline|Timeline`)
        (:`Update`
          (`SceneComponent.K2_AddLocalRotation` (`self.Cube1`) (`KismetMathLibrary.RLerp` (struct) (struct :`Pitch` 90.0) _delta) false false)
          (for _array_element (`self.TRIGGER`)
            (`self.SetActorHiddenInGame` _array_element false))
          (`/Game/10_BLUEPRINT/14_INTERACTIBLE/UTILITIES/BP_Text.ShowText` (`self.Text`))
          (`KismetSystemLibrary.Delay` (`self.Delay Text Next`))
          (for _array_element_2 (`self.TextNext`)
            (`/Game/10_BLUEPRINT/14_INTERACTIBLE/UTILITIES/BP_Text.ShowText` _array_element_2)))))))

(fn `UserConstructionScript`
  (`parent.UserConstructionScript`))