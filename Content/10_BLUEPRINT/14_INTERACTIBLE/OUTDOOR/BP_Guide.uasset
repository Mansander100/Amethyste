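; BP_Guide is an outdoor interactible guide that shows text to the player when interacted with.
; InteractionB calls FindText, which uses GeneralManager's CurrentIndex to pick a data table row and returns its first Text entry for BPText to display.
; When BP_CHARACTER leaves the sphere, the text is reset to empty.
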(event `self.InteractionB`
  (params (Player :type "/Game/10_BLUEPRINT/12_CONTROLLER/BP_CHARACTER Object Reference"))
  (bind _bp_text (`self.BP_Text`))
  (bind _return (`self.Find Text`))
  (set `/Game/10_BLUEPRINT/14_INTERACTIBLE/UTILITIES/BP_Text.Text` _return _bp_text)
  (`/Game/10_BLUEPRINT/14_INTERACTIBLE/UTILITIES/BP_Text.ShowText` _bp_text))

(event `self.Sphere.OnComponentEndOverlap`
  (params (OverlappedComponent :type "PrimitiveComponent Object Reference") (OtherActor :type "Actor Object Reference") (OtherComp :type "PrimitiveComponent Object Reference") (OtherBodyIndex :type Integer))
  (bind _bp_text (`self.BP_Text`))
  (if (== (`GameplayStatics.GetObjectClass` OtherActor) "/Game/10_BLUEPRINT/12_CONTROLLER/BP_CHARACTER.BP_CHARACTER_C")
    (set `/Game/10_BLUEPRINT/14_INTERACTIBLE/UTILITIES/BP_Text.Text` "" _bp_text)
    (`/Game/10_BLUEPRINT/14_INTERACTIBLE/UTILITIES/BP_Text.ShowText` _bp_text)))

(fn `Find Text`
  (returns (Return :type Text))
  (bind _datatable (`self.DataTable`))
  (bind _outrownames (`DataTableFunctionLibrary.GetDataTableRowNames` _datatable))
  (bind _returnvalue (`|GetDataTableRow` _datatable (`|GetArrayItem` _outrownames (`/Game/10_BLUEPRINT/15_MANAGER/BP_GeneralManager.current index` (`self.GeneralManager`))))
    (:`then`
      (return (`|GetArrayItem` (`.Text_9_7007BD924A4FCA4C5B5BCFB1F1D7C6B6` (break `/Game/10_BLUEPRINT/18_PARAMETERS/STRUCTURE/TextData` _returnvalue)))))))

(fn `UserConstructionScript`
  (`parent.UserConstructionScript`))