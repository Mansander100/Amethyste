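; BP_Text is an actor that reveals its text in a TextRender component with a typewriter effect when play begins.
; ShowText walks the characters of Text through a delayed loop macro, appending each to DisplayText and refreshing the render every 0.05 seconds.
; The "§" character is not drawn, so it acts as a one-step pause in the reveal.
; HideText hides the whole actor in game.
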(event `self.ReceiveBeginPlay`
  (`TextRenderComponent.K2_SetText` (`self.TextRender`) (`KismetTextLibrary.Conv_StringToText` (`self.displayText`)))
  (`self.ShowText`))

(event `ShowText`
  (bind _returnvalue (`KismetStringLibrary.GetCharacterArrayFromString` (`KismetTextLibrary.Conv_TextToString` (`self.Text`))))
  (bind _index (`self.ForLoopWithBreakAndDelay` 0 (`KismetArrayLibrary.Array_Length` _returnvalue) 0.05)
    (:`LoopBody`
      (bind _output (`|GetArrayItem` _returnvalue _index))
      (if (not (`KismetStringLibrary.EqualEqual_StrStr` _output "§"))
        (bind _output_get (set `self.displayText` (`KismetStringLibrary.Concat_StrStr` (`self.displayText`) _output)))
        (`TextRenderComponent.K2_SetText` (`self.TextRender`) (`KismetTextLibrary.Conv_StringToText` _output_get))
        (else
          (bind _output_get_2 (set `self.displayText` (`KismetStringLibrary.Concat_StrStr` (`self.displayText`) " \n")))
          (`TextRenderComponent.K2_SetText` (`self.TextRender`) (`KismetTextLibrary.Conv_StringToText` _output_get_2)))))))

(event `HideText`
  (`self.SetActorHiddenInGame` true))

(fn `UserConstructionScript`)