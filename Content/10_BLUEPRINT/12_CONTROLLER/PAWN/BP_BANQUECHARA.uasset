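; BP_BANQUECHARA is a player pawn with a cine camera that looks around and rides along splines.
; Each tick it line-traces from the camera for interactable detection and follows any spline assigned through StartMoving or NewPath.
; Its PlayerController reference receives detection hits and interaction inputs A/B/C, and is possessed when Unpos destroys this pawn.
; The logic clearing a finished spline is disconnected.
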(event `self.ReceiveTick`
  (params (DeltaSeconds :type "Float (single-precision)"))
  (bind _splinetomove (`self.SplineToMove`))
  (`|ExecutionSequence`
    (:`then_0`
      (bind _outhit (`self.Draw Camera Raycast` 10000.0)
        (:`Output`
          (`/Game/10_BLUEPRINT/12_CONTROLLER/BP_CHARACTER.Detect Interactible Object` (`self.PlayerController`) _outhit))))
    (:`then_1`
      (if (!= _splinetomove null)
        (`self.MoveWithASpline` _splinetomove DeltaSeconds)))))

(event `EnhancedInput|/Game/10_BLUEPRINT/18_PARAMETERS/INPUT/Actions/IA_Look`
  (params (ActionValue :type "Vector2D Structure") (ElapsedSeconds :type "Float (double-precision)") (TriggeredSeconds :type "Float (double-precision)") (InputAction :type "InputAction Object Reference" :default "/Game/10_BLUEPRINT/18_PARAMETERS/INPUT/Actions/IA_Look.IA_Look"))
  (:`Triggered`
    (`self.AddControllerYawInput` (* ActionValue_X 1.0))
    (`self.AddControllerPitchInput` (* ActionValue_Y 1.0))))

(event `MoveWithASpline`
  (params (SplinePath :type "/Game/10_BLUEPRINT/14_INTERACTIBLE/OBJECT_AMETHYSTE/SouvenirPrincipal/BP_Spline Object Reference") (DeltaTime :type "Float (double-precision)"))
  (`/Engine/EditorBlueprintResources/StandardMacros.IsValid` SplinePath
    (:`Is Valid`
      (bind (_transformalongthespline _finish) (`/Game/10_BLUEPRINT/14_INTERACTIBLE/OBJECT_AMETHYSTE/SouvenirPrincipal/BP_Spline.GetTransformAlongTheSpline` SplinePath DeltaTime))
      (`SceneComponent.K2_SetWorldTransform` (`self.Capsule`) _transformalongthespline false false))))

(event `NewPath`
  (params (path :type "/Game/10_BLUEPRINT/14_INTERACTIBLE/OBJECT_AMETHYSTE/SouvenirPrincipal/BP_Spline Object Reference"))
  (set `self.SplineToMove` path))

(event `Unpos`
  (bind _returnvalue (`GameplayStatics.GetPlayerController` 0))
  ;[0 0 0] Unposses
  (`Controller.UnPossess` _returnvalue)
  (`Controller.Possess` _returnvalue (`self.PlayerController`))
  (`self.K2_DestroyActor`))

(event `EnhancedInput|/Game/10_BLUEPRINT/18_PARAMETERS/INPUT/Actions/IA_interactionA`
  (params (ActionValue :type Boolean) (ElapsedSeconds :type "Float (double-precision)") (TriggeredSeconds :type "Float (double-precision)") (InputAction :type "InputAction Object Reference" :default "/Game/10_BLUEPRINT/18_PARAMETERS/INPUT/Actions/IA_interactionA.IA_interactionA"))
  (:`Triggered`
    (`/Game/10_BLUEPRINT/12_CONTROLLER/BP_CHARACTER.InputA` (`self.PlayerController`))))

(event `EnhancedInput|/Game/10_BLUEPRINT/18_PARAMETERS/INPUT/Actions/IA_interactionB`
  (params (ActionValue :type Boolean) (ElapsedSeconds :type "Float (double-precision)") (TriggeredSeconds :type "Float (double-precision)") (InputAction :type "InputAction Object Reference" :default "/Game/10_BLUEPRINT/18_PARAMETERS/INPUT/Actions/IA_interactionB.IA_interactionB"))
  (:`Triggered`
    (`/Game/10_BLUEPRINT/12_CONTROLLER/BP_CHARACTER.InputB` (`self.PlayerController`))))

(event `EnhancedInput|/Game/10_BLUEPRINT/18_PARAMETERS/INPUT/Actions/IA_interactionC`
  (params (ActionValue :type Boolean) (ElapsedSeconds :type "Float (double-precision)") (TriggeredSeconds :type "Float (double-precision)") (InputAction :type "InputAction Object Reference" :default "/Game/10_BLUEPRINT/18_PARAMETERS/INPUT/Actions/IA_interactionC.IA_interactionC"))
  (:`Triggered`
    (`/Game/10_BLUEPRINT/12_CONTROLLER/BP_CHARACTER.Input C` (`self.PlayerController`))))

(fn `StartMoving`
  (params (Spline :type "/Game/10_BLUEPRINT/14_INTERACTIBLE/OBJECT_AMETHYSTE/SouvenirPrincipal/BP_Spline Object Reference"))
  (set `self.SplineToMove` Spline)
  (return))

(fn `UserConstructionScript`)