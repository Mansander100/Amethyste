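; BP_Guide is an interactable guide that shows dialogue tied to the current index held by GeneralManager.
; InteractionB asks the manager to show the dialogue two entries past that index for a few seconds.
; A separate FindText function reads the data table row at the unshifted index by row-name order and returns its first text entry, though nothing in this graph calls it.
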(event `self.InteractionB`
  (params (Player :type "/Game/10_BLUEPRINT/12_CONTROLLER/BP_CHARACTER Object Reference"))
  (`/Game/10_BLUEPRINT/15_MANAGER/BP_GeneralManager.ShowDialogue` :`self` (`self.GeneralManager`) :`index` (+ (`/Game/10_BLUEPRINT/15_MANAGER/BP_GeneralManager.current index` (`self.GeneralManager`)) 2) :`Duration` 5.0))

(fn `Find Text`
  (returns (Return :type Text))
  (bind _datatable (`self.DataTable`))
  (bind _outrownames (`DataTableFunctionLibrary.GetDataTableRowNames` _datatable))
  (bind _returnvalue (`|GetDataTableRow` _datatable (`|GetArrayItem` _outrownames (`/Game/10_BLUEPRINT/15_MANAGER/BP_GeneralManager.current index` (`self.GeneralManager`))))
    (:`then`
      (return (`|GetArrayItem` (`.Text_9_7007BD924A4FCA4C5B5BCFB1F1D7C6B6` (break `/Game/10_BLUEPRINT/18_PARAMETERS/STRUCTURE/TextData` _returnvalue)))))))

(fn `UserConstructionScript`
  (`parent.UserConstructionScript`))