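; BP_TriggerBlockObject is a trigger volume that keeps important BP_Child objects inside its box by sending them back to base when they exit.
; On end overlap, it calls InteractionB if the object's player is grabbing.
; Otherwise, if the object is being inspected, it clears that state and restores the player's movement, look and mesh collision, with gravity off.
; It then calls ReturnToBase on the object and plays audio.
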(event `self.Box.OnComponentEndOverlap`
  (params (OverlappedComponent :type "PrimitiveComponent Object Reference") (OtherActor :type "Actor Object Reference") (OtherComp :type "PrimitiveComponent Object Reference") (OtherBodyIndex :type Integer))
  (if (`KismetMathLibrary.ClassIsChildOf` (`GameplayStatics.GetObjectClass` OtherActor) "/Game/10_BLUEPRINT/14_INTERACTIBLE/OBJECT_AMETHYSTE/BP_Child.BP_Child_C")
    (bind _asbp_child (cast `/Game/10_BLUEPRINT/14_INTERACTIBLE/OBJECT_AMETHYSTE/BP_Child` OtherActor))
    (if (`/Game/10_BLUEPRINT/14_INTERACTIBLE/OBJECT_AMETHYSTE/BP_Child.IsImportant` _asbp_child)
      (bind _player (`/Game/10_BLUEPRINT/14_INTERACTIBLE/OBJECT_AMETHYSTE/BP_Child.Player` _asbp_child))
      (if (`/Game/10_BLUEPRINT/12_CONTROLLER/BP_CHARACTER.IsGrabbingObject` _player)
        (`/Game/10_BLUEPRINT/14_INTERACTIBLE/OBJECT_AMETHYSTE/BP_ParentObject.InteractionB` _asbp_child _player)
        (elif (`/Game/10_BLUEPRINT/14_INTERACTIBLE/OBJECT_AMETHYSTE/BP_Child.isInspecting` _asbp_child)
          (set `/Game/10_BLUEPRINT/12_CONTROLLER/BP_CHARACTER.canMove` true _player)
          (set `/Game/10_BLUEPRINT/12_CONTROLLER/BP_CHARACTER.canLook` true _player)
          (set `/Game/10_BLUEPRINT/12_CONTROLLER/BP_CHARACTER.IsGrabbingObject` false _player)
          (set `/Game/10_BLUEPRINT/14_INTERACTIBLE/OBJECT_AMETHYSTE/BP_Child.isInspecting` false _asbp_child)
          (bind _mesh (`Character.Mesh` _player))
          (`PrimitiveComponent.SetCollisionEnabled` _mesh "QueryAndPhysics")
          (`PrimitiveComponent.SetEnableGravity` _mesh false)))
      (`/Game/10_BLUEPRINT/14_INTERACTIBLE/OBJECT_AMETHYSTE/BP_Child.Return To Base` _asbp_child)
      (`AudioComponent.Play` (`self.Audio`) 0.0))))

(fn `UserConstructionScript`)