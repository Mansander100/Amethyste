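; BP_ReminiscenceManager drives an ordered reminiscence sequence, advancing only when the actor passed in matches the expected object at the current ActionList index.
; A match runs that step's actions, which show BP_Text or activate and deactivate actors by toggling visibility and collision, then increments the index.
; The check exists as both an event and a near-identical function that also returns whether the actor matched.
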(event `CheckRightAction?`
  (params (Actor :type "Actor Object Reference"))
  (bind (_objecttype _action) (break `/Game/10_BLUEPRINT/18_PARAMETERS/STRUCTURE/ActionStrct` (`|GetArrayItem` (`self.ActionList`) (`self.Index`))))
  (if (== Actor _objecttype)
    (for _array_element _action
      (bind (_object _type) (break `/Game/10_BLUEPRINT/18_PARAMETERS/STRUCTURE/ActionType` _array_element))
      (switch `/Game/10_BLUEPRINT/18_PARAMETERS/ENUMERATION/ActionType` _type
        (:`NewEnumerator0`
          (`self.ShowText` _object))
        (:`NewEnumerator1`
          (`self.Activate` _object))
        (:`NewEnumerator2`
          (`self.Deactivate` _object))))
    (`/Engine/EditorBlueprintResources/StandardMacros.IncrementInt` (`self.Index`))))

(fn `Activate`
  (params (Actor :type "Actor Object Reference"))
  (`self.SetActorHiddenInGame` Actor false)
  (`self.SetActorEnableCollision` Actor true))

(fn `CheckRightAction`
  (params (Actor :type "Actor Object Reference"))
  (returns (`yes?` :type Boolean))
  (bind (_objecttype _action) (break `/Game/10_BLUEPRINT/18_PARAMETERS/STRUCTURE/ActionStrct` (`|GetArrayItem` (`self.ActionList`) (`self.Index`))))
  (if (== Actor _objecttype)
    (for _array_element _action
      (bind (_object _type) (break `/Game/10_BLUEPRINT/18_PARAMETERS/STRUCTURE/ActionType` _array_element))
      (switch `/Game/10_BLUEPRINT/18_PARAMETERS/ENUMERATION/ActionType` _type
        (:`NewEnumerator0`
          (`self.ShowText` _object))
        (:`NewEnumerator1`
          (`self.Activate` _object))
        (:`NewEnumerator2`
          (`self.Deactivate` _object))))
    (`/Engine/EditorBlueprintResources/StandardMacros.IncrementInt` (`self.Index`)
      (:`  `
        (return true)))
    (else
      (return false))))

(fn `Deactivate`
  (params (Actor :type "Actor Object Reference"))
  (`self.SetActorHiddenInGame` Actor true)
  (`self.SetActorEnableCollision` Actor false))

(fn `ShowText`
  (params (Actor :type "Actor Object Reference"))
  (bind _asbp_text (cast `/Game/10_BLUEPRINT/14_INTERACTIBLE/UTILITIES/BP_Text` Actor))
  (`/Game/10_BLUEPRINT/14_INTERACTIBLE/UTILITIES/BP_Text.ShowText` _asbp_text))

(fn `UserConstructionScript`)