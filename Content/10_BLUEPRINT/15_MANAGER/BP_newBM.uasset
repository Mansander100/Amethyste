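; Manager for the bank sequence, enabling its trigger on StartBank and driving the scene's branching choices from a data table.
; NextChoice uses an index to fetch a row, plays its optional level sequence, then hides and updates five interaction actors (C1, C2, Banquier, Plafond, Porte).
; After the row's delay, it moves the General actor if a new player position is set and re-shows the interactions.
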(event `self.ReceiveBeginPlay`
  (`self.SetActorEnableCollision` (`self.Trigger`) false))

(event `StartBank`
  (`self.SetActorEnableCollision` (`self.Trigger`) true))

(event `NextChoice`
  (params (NewIndex :type Integer))
  (bind _output_get (set `self.index` NewIndex))
  (bind _returnvalue (`|GetDataTableRow` (`self.DATA TABLE`) (`|GetArrayItem` (`self.TableName`) (- _output_get 1)))
    (:`then`
      (bind (_animation _delay _newplayerpos _c1 _c2 _banquier _plafond _porte) (break `/Game/10_BLUEPRINT/18_PARAMETERS/STRUCTURE/Banque/Possibilities` _returnvalue))
      (`/Engine/EditorBlueprintResources/StandardMacros.IsValid` _animation
        (:`Is Valid`
          (bind (_outactor _returnvalue_2) (`LevelSequencePlayer.CreateLevelSequencePlayer` _animation))
          (`MovieSceneSequencePlayer.Play` _returnvalue_2))
        (:`Is Not Valid`
          _))
      (set `self.NewChoice` (`|MakeArray` _c1 _c2 _banquier _plafond _porte))
      (for (_array_element _array_index) (`self.AllInteractionList`)
        (`PrimitiveComponent.SetCollisionEnabled` (`/Game/10_BLUEPRINT/14_INTERACTIBLE/OBJECT_AMETHYSTE/SouvenirPrincipal/BP_BanqueTest.Cylinder` _array_element) "NoCollision")
        (`self.SetActorHiddenInGame` _array_element true)
        (`/Game/10_BLUEPRINT/14_INTERACTIBLE/OBJECT_AMETHYSTE/SouvenirPrincipal/BP_InteractionBank.ChangeData` _array_element (`|GetArrayItem` (`self.NewChoice`) _array_index)))
      (`KismetSystemLibrary.Delay` _delay)
      (if (`KismetMathLibrary.NotEqualExactly_VectorVector` _newplayerpos)
        (`self.K2_SetActorLocation` (`self.General`) _newplayerpos false false))
      (for _array_element_2 (`self.AllInteractionList`)
        (`PrimitiveComponent.SetCollisionEnabled` (`/Game/10_BLUEPRINT/14_INTERACTIBLE/OBJECT_AMETHYSTE/SouvenirPrincipal/BP_BanqueTest.Cylinder` _array_element_2) "QueryOnly")
        (`self.SetActorHiddenInGame` _array_element_2 false)))))

(fn `UserConstructionScript`
  (set `self.AllInteractionList` (`|MakeArray` (`self.C1`) (`self.C2`) (`self.Banquier`) (`self.Plafond`) (`self.Porte`)))
  (bind _outrownames (`DataTableFunctionLibrary.GetDataTableRowNames` (`self.DATA TABLE`)))
  (set `self.TableName` _outrownames))