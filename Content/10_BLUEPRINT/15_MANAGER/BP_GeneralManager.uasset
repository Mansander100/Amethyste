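; BP_GeneralManager sequences the game's scenario through an ordered list of steps, each pairing a trigger object with the games it starts.
; NextStepInScenario advances only when the caller matches the current trigger, activating that step's reminiscence managers or starting its BP_newBM banks.
; ReminiscenceEnd counts finished reminiscences and, once the target count is reached, passes the manager itself as the next trigger.
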(fn `Next Step in Scenario`
  (params (Object :type "Actor Object Reference"))
  (bind (_output_declacheur _output_game) (break `/Game/10_BLUEPRINT/18_PARAMETERS/STRUCTURE/GeneralManager/GameOrder` (`|GetArrayItem` (`self.Order`) (`self.current index`))))
  (if (== Object _output_declacheur)
    (for _array_element (`self.AllGame`)
      (if (`KismetArrayLibrary.Array_Contains` _output_game _array_element)
        (`KismetSystemLibrary.PrintString` (`KismetSystemLibrary.GetDisplayName` _array_element))
        (bind _asbp_reminiscence_manager (cast `/Game/10_BLUEPRINT/15_MANAGER/BP_ReminiscenceManager` _array_element)
          (:`then`
            (`/Game/10_BLUEPRINT/15_MANAGER/BP_ReminiscenceManager.ActivateRemi` _asbp_reminiscence_manager))
          (:`CastFailed`
            (bind _asbp_new_bm (cast `/Game/10_BLUEPRINT/15_MANAGER/BP_newBM` _array_element))
            (`/Game/10_BLUEPRINT/15_MANAGER/BP_newBM.StartBank` _asbp_new_bm)))))
    (`/Engine/EditorBlueprintResources/StandardMacros.IncrementInt` (`self.current index`))))

(fn `ReminiscenceEnd`
  (`/Engine/EditorBlueprintResources/StandardMacros.IncrementInt` (`self.ReminiscenceFini`)
    (:`  `
      (if (not (< (`self.ReminiscenceFini`) (`self.NbReminiscence`)))
        (`self.Next Step in Scenario` self)))))

(fn `UserConstructionScript`)