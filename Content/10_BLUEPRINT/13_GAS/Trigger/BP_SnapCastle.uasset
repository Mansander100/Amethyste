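; BP_SnapCastle is a snap target that pulls a passed-in object's mesh into place at its Box, likely a castle piece given the name.
; An externally called Snap event plays a timeline, lerping the mesh from its current transform each update toward the Box's location and rotation at unit scale.
; The same updates activate the Congrats effect, unhide Niagara1 and disable the Box's collision.
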(event `self.Snap`
  (params (Object :type "/Game/10_BLUEPRINT/14_INTERACTIBLE/OBJECT_AMETHYSTE/BP_Child Object Reference"))
  (bind _mesh (`/Game/10_BLUEPRINT/14_INTERACTIBLE/OBJECT_AMETHYSTE/BP_ParentObject.Mesh` Object))
  (bind (_returnvalue_location _returnvalue_rotation) (`KismetMathLibrary.BreakTransform` (`SceneComponent.K2_GetComponentToWorld` (`self.Box`))))
  (bind (_direction _delta) (`Timeline|Timeline`)
    (:`Update`
      (`SceneComponent.K2_SetWorldTransform` _mesh (`KismetMathLibrary.TLerp` (`SceneComponent.K2_GetComponentToWorld` _mesh) (`KismetMathLibrary.MakeTransform` _returnvalue_location _returnvalue_rotation) _delta) false false)
      (`ActorComponent.Activate` (`self.Congrats`) false)
      (`SceneComponent.SetHiddenInGame` (`self.Niagara1`) false false)
      (`PrimitiveComponent.SetCollisionEnabled` (`self.Box`) "NoCollision"))))

(fn `UserConstructionScript`
  (`parent.UserConstructionScript`))