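; BP_CollectZone_NotAND is a trigger zone that drives its ACSInteraction component when designated objects enter or leave its Box.
; On a non-character begin overlap while the zone is not hidden, it starts the interaction if any ObjectToPlace entry is inside, so not all are required.
; Any listed BP_Child leaving stops the interaction, without checking for others still inside.
; Debug prints remain in the overlap check.
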(event `self.Box.OnComponentBeginOverlap`
  (params (OverlappedComponent :type "PrimitiveComponent Object Reference") (OtherActor :type "Actor Object Reference") (OtherComp :type "PrimitiveComponent Object Reference") (OtherBodyIndex :type Integer) (bFromSweep :type Boolean) (SweepResult :type "HitResult Structure (by ref)"))
  (if (and (!= (`GameplayStatics.GetObjectClass` OtherActor) "/Game/10_BLUEPRINT/12_CONTROLLER/BP_CHARACTER.BP_CHARACTER_C") (not (`self.bHidden`)))
    (`KismetSystemLibrary.PrintString` "Hello")
    (set `self.On` false)
    (for _array_element (`self.ObjectToPlace`)
      (if (`KismetArrayLibrary.Array_Contains` (`PrimitiveComponent.GetOverlappingActors` (`self.Box`) "/Script/Engine.Actor") _array_element)
        (set `self.On` true)
        (`KismetSystemLibrary.PrintString` "not good")))
    (if (`self.On`)
      (`/Game/10_BLUEPRINT/13_GAS/ACS_Interaction.Start_Interaction` (`self.ACS_Interaction`)))))

(event `self.Box.OnComponentEndOverlap`
  (params (OverlappedComponent :type "PrimitiveComponent Object Reference") (OtherActor :type "Actor Object Reference") (OtherComp :type "PrimitiveComponent Object Reference") (OtherBodyIndex :type Integer))
  (if (!= (`GameplayStatics.GetObjectClass` OtherActor) "/Game/10_BLUEPRINT/12_CONTROLLER/BP_CHARACTER.BP_CHARACTER_C")
    (set `self.On` true)
    (bind _asbp_child (cast `/Game/10_BLUEPRINT/14_INTERACTIBLE/OBJECT_AMETHYSTE/BP_Child` OtherActor))
    (if (`KismetArrayLibrary.Array_Contains` (`self.ObjectToPlace`) _asbp_child)
      (`/Game/10_BLUEPRINT/13_GAS/ACS_Interaction.Stop_Interaction` (`self.ACS_Interaction`)))))

(fn `UserConstructionScript`)