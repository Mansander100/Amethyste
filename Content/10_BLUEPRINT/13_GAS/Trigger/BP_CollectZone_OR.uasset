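; BP_CollectZone_OR is a trigger zone that activates when any object from its ObjectToPlace list is placed inside it.
; On BeginPlay, it copies the first object's mesh to its Cube and sizes the Box from that mesh's bounds.
; Non-character overlaps start ACSInteraction and hide the Cube if a listed object is inside.
; Any listed BP_Child leaving stops the interaction and shows the Cube, without checking remaining objects.
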(event `self.Box.OnComponentBeginOverlap`
  (params (OverlappedComponent :type "PrimitiveComponent Object Reference") (OtherActor :type "Actor Object Reference") (OtherComp :type "PrimitiveComponent Object Reference") (OtherBodyIndex :type Integer) (bFromSweep :type Boolean) (SweepResult :type "HitResult Structure (by ref)"))
  (if (!= (`GameplayStatics.GetObjectClass` OtherActor) "/Game/10_BLUEPRINT/12_CONTROLLER/BP_CHARACTER.BP_CHARACTER_C")
    (set `self.On` false)
    (for _array_element (`self.ObjectToPlace`)
      (if (`KismetArrayLibrary.Array_Contains` (`PrimitiveComponent.GetOverlappingActors` (`self.Box`) "/Script/Engine.Actor") _array_element)
        (set `self.On` true)))
    (if (`self.On`)
      (`/Game/10_BLUEPRINT/13_GAS/ACS_Interaction.Start_Interaction` (`self.ACS_Interaction`))
      (`SceneComponent.SetHiddenInGame` (`self.Cube`) true false))))

(event `self.Box.OnComponentEndOverlap`
  (params (OverlappedComponent :type "PrimitiveComponent Object Reference") (OtherActor :type "Actor Object Reference") (OtherComp :type "PrimitiveComponent Object Reference") (OtherBodyIndex :type Integer))
  (if (!= (`GameplayStatics.GetObjectClass` OtherActor) "/Game/10_BLUEPRINT/12_CONTROLLER/BP_CHARACTER.BP_CHARACTER_C")
    (set `self.On` false)
    (bind _asbp_child (cast `/Game/10_BLUEPRINT/14_INTERACTIBLE/OBJECT_AMETHYSTE/BP_Child` OtherActor))
    (if (`KismetArrayLibrary.Array_Contains` (`self.ObjectToPlace`) _asbp_child)
      (set `self.On` true)
      (`/Game/10_BLUEPRINT/13_GAS/ACS_Interaction.Stop_Interaction` (`self.ACS_Interaction`))
      (`SceneComponent.SetHiddenInGame` (`self.Cube`) false false))))

(event `self.ReceiveBeginPlay`
  (bind _staticmesh (`StaticMeshComponent.StaticMesh` (`/Game/10_BLUEPRINT/14_INTERACTIBLE/OBJECT_AMETHYSTE/BP_Child.Cube` (`|GetArrayItem` (`self.ObjectToPlace`)))))
  (bind (_returnvalue_min _returnvalue_max _returnvalue_isvalid) (break `Box` (`StaticMesh.GetBoundingBox` _staticmesh)))
  (`StaticMeshComponent.SetStaticMesh` (`self.Cube`) _staticmesh)
  (`BoxComponent.SetBoxExtent` (`self.Box`) _returnvalue_max _returnvalue_isvalid))

(fn `UserConstructionScript`)