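; Trigger zone that snaps one designated object, ObjectToPlace, into place at its Box.
; If the player is still grabbing the object on overlap, the zone registers itself in the BP_Child's Snap variable, cleared on exit; otherwise it snaps immediately.
; Snap runs a timeline that lerps the mesh to the Box's location and rotation at unit scale, disabling its collision and activating Congrats.
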(event `Snap`
  (params (Object :type "/Game/10_BLUEPRINT/14_INTERACTIBLE/OBJECT_AMETHYSTE/BP_Child Object Reference"))
  (bind _mesh (`/Game/10_BLUEPRINT/14_INTERACTIBLE/OBJECT_AMETHYSTE/BP_ParentObject.Mesh` Object))
  (bind (_returnvalue_location _returnvalue_rotation) (`KismetMathLibrary.BreakTransform` (`SceneComponent.K2_GetComponentToWorld` (`self.Box`))))
  (bind (_direction _delta) (`Timeline|Timeline_0`)
    (:`Update`
      (`SceneComponent.K2_SetWorldTransform` _mesh (`KismetMathLibrary.TLerp` (`SceneComponent.K2_GetComponentToWorld` _mesh) (`KismetMathLibrary.MakeTransform` _returnvalue_location _returnvalue_rotation) _delta) false false)
      (`PrimitiveComponent.SetCollisionEnabled` _mesh "NoCollision")
      (`ActorComponent.Activate` (`self.Congrats`) false))))

(event `self.Box.OnComponentBeginOverlap`
  (params (OverlappedComponent :type "PrimitiveComponent Object Reference") (OtherActor :type "Actor Object Reference") (OtherComp :type "PrimitiveComponent Object Reference") (OtherBodyIndex :type Integer) (bFromSweep :type Boolean) (SweepResult :type "HitResult Structure (by ref)"))
  (if (!= (`GameplayStatics.GetObjectClass` OtherActor) "/Game/10_BLUEPRINT/12_CONTROLLER/BP_CHARACTER.BP_CHARACTER_C")
    (for _array_element (`PrimitiveComponent.GetOverlappingActors` (`self.Box`) "/Script/Engine.Actor")
      (if (== _array_element (`self.ObjectToPlace`))
        (bind _asbp_child (cast `/Game/10_BLUEPRINT/14_INTERACTIBLE/OBJECT_AMETHYSTE/BP_Child` _array_element))
        (if (`/Game/10_BLUEPRINT/12_CONTROLLER/BP_CHARACTER.IsGrabbingObject` (`/Game/10_BLUEPRINT/14_INTERACTIBLE/OBJECT_AMETHYSTE/BP_Child.Player` _asbp_child))
          (set `/Game/10_BLUEPRINT/14_INTERACTIBLE/OBJECT_AMETHYSTE/BP_Child.Snap` self _asbp_child)
          (else
            (`self.Snap` _asbp_child)))))))

(event `self.Box.OnComponentEndOverlap`
  (params (OverlappedComponent :type "PrimitiveComponent Object Reference") (OtherActor :type "Actor Object Reference") (OtherComp :type "PrimitiveComponent Object Reference") (OtherBodyIndex :type Integer))
  (if (and (!= (`GameplayStatics.GetObjectClass` OtherActor) "/Game/10_BLUEPRINT/12_CONTROLLER/BP_CHARACTER.BP_CHARACTER_C") (== OtherActor (`self.ObjectToPlace`)))
    (bind _asbp_child (cast `/Game/10_BLUEPRINT/14_INTERACTIBLE/OBJECT_AMETHYSTE/BP_Child` OtherActor))
    (set `/Game/10_BLUEPRINT/14_INTERACTIBLE/OBJECT_AMETHYSTE/BP_Child.Snap` null _asbp_child)))

(event `self.ReceiveBeginPlay`)

(fn `UserConstructionScript`)