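; BP_BANQUECHARA is a character that rides along an assigned spline path while the player can still look around.
; Each Tick, it snaps the capsule to the transform the SplineToMove object returns for the frame's delta time, without sweeping.
; When the path reports it is finished, SplineToMove is cleared and movement stops.
; Enhanced Input IA_Look drives controller yaw and pitch independently of that movement.
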(event `self.ReceiveTick`
  (params (DeltaSeconds :type "Float (single-precision)"))
  (`self.MoveWithASpline` (`self.SplineToMove`) DeltaSeconds))

(event `EnhancedInput|/Game/FirstPerson/Input/Actions/IA_Look`
  (params (ActionValue :type "Vector2D Structure") (ElapsedSeconds :type "Float (double-precision)") (TriggeredSeconds :type "Float (double-precision)") (InputAction :type "InputAction Object Reference" :default "/Game/FirstPerson/Input/Actions/IA_Look.IA_Look"))
  (:`Triggered`
    (`self.AddControllerYawInput` (* ActionValue_X 1.0))
    (`self.AddControllerPitchInput` (* ActionValue_Y 1.0))))

(event `MoveWithASpline`
  (params (SplinePath :type "/Game/OBJECT_AMETHYSTE/SouvenirPrincipal/BP_Spline Object Reference") (DeltaTime :type "Float (double-precision)"))
  (`/Engine/EditorBlueprintResources/StandardMacros.IsValid` SplinePath
    (:`Is Valid`
      (bind (_transformalongthespline _finish) (`/Game/OBJECT_AMETHYSTE/SouvenirPrincipal/BP_Spline.GetTransformAlongTheSpline` SplinePath DeltaTime))
      (`SceneComponent.K2_SetWorldTransform` (`self.Capsule`) _transformalongthespline false false)
      (if _finish
        (set `self.SplineToMove` null)))))

(fn `UserConstructionScript`)