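; BP_CollectZone is a trigger zone that drives an interaction based on whether a set of required objects is inside its box.
; On each begin overlap, it checks that every ObjectToPlace entry is among the Box's overlapping actors.
; It starts ACSInteraction when all are present and stops it otherwise.
; End overlap is not handled, so removing an object does not itself trigger a recheck.
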(event `self.Box.OnComponentBeginOverlap`
  (params (OverlappedComponent :type "PrimitiveComponent Object Reference") (OtherActor :type "Actor Object Reference") (OtherComp :type "PrimitiveComponent Object Reference") (OtherBodyIndex :type Integer) (bFromSweep :type Boolean) (SweepResult :type "HitResult Structure (by ref)"))
  (bind _acs_interaction (`self.ACS_Interaction`))
  (set `self.On` true)
  (for _array_element (`self.ObjectToPlace`)
    (if (not (`KismetArrayLibrary.Array_Contains` (`PrimitiveComponent.GetOverlappingActors` (`self.Box`) "/Script/Engine.Actor") _array_element))
      (set `self.On` false)))
  (if (`self.On`)
    (`/Game/GAS/ACS_Interaction.Start_Interaction` _acs_interaction)
    (else
      (`/Game/GAS/ACS_Interaction.Stop_Interaction` _acs_interaction))))

(fn `UserConstructionScript`)