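; Trigger zone that activates an interaction once every object in its ObjectToPlace list is inside its box, acting as an AND condition.
; Each non-character begin overlap checks the whole list against the box's overlapping actors, then starts ACSInteraction and hides the Cube if all are present.
; When any listed BP_ParentObject leaves, it stops the interaction and shows the Cube again.
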(event `self.Box.OnComponentBeginOverlap`
  (params (OverlappedComponent :type "PrimitiveComponent Object Reference") (OtherActor :type "Actor Object Reference") (OtherComp :type "PrimitiveComponent Object Reference") (OtherBodyIndex :type Integer) (bFromSweep :type Boolean) (SweepResult :type "HitResult Structure (by ref)"))
  (if (!= (`GameplayStatics.GetObjectClass` OtherActor) "/Game/CHARACTER_AMETHYSTE/Blueprints/BP_CHARACTER.BP_CHARACTER_C")
    (set `self.On` true)
    (for _array_element (`self.ObjectToPlace`)
      (if (not (`KismetArrayLibrary.Array_Contains` (`PrimitiveComponent.GetOverlappingActors` (`self.Box`) "/Script/Engine.Actor") _array_element))
        (set `self.On` false)))
    (if (`self.On`)
      (`/Game/GAS/ACS_Interaction.Start_Interaction` (`self.ACS_Interaction`))
      (`SceneComponent.SetHiddenInGame` (`self.Cube`) true false))))

(event `self.Box.OnComponentEndOverlap`
  (params (OverlappedComponent :type "PrimitiveComponent Object Reference") (OtherActor :type "Actor Object Reference") (OtherComp :type "PrimitiveComponent Object Reference") (OtherBodyIndex :type Integer))
  (if (!= (`GameplayStatics.GetObjectClass` OtherActor) "/Game/CHARACTER_AMETHYSTE/Blueprints/BP_CHARACTER.BP_CHARACTER_C")
    (set `self.On` true)
    (bind _asbp_parent_object (cast `/Game/OBJECT_AMETHYSTE/BP_ParentObject` OtherActor))
    (if (`KismetArrayLibrary.Array_Contains` (`self.ObjectToPlace`) _asbp_parent_object)
      (`/Game/GAS/ACS_Interaction.Stop_Interaction` (`self.ACS_Interaction`))
      (`SceneComponent.SetHiddenInGame` (`self.Cube`) false false))))

(fn `UserConstructionScript`)