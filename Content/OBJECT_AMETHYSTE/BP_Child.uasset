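; Child Blueprint of an interactable object that the player can inspect up close or carry.
; InteractionA toggles inspection, locking player movement and look while a Zoom timeline lerps the Cube to the player's Arrow1, then reverses to restore collision and gravity.
; During inspection the Inspect event's X/Y input rotates the Cube locally.
; InteractionB uses a FlipFlop to grab and release the player's current interactible through its PhysicsHandle.
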(event `Inspect`
  (params (X :type "Float (double-precision)") (Y :type "Float (double-precision)"))
  (`SceneComponent.K2_AddLocalRotation` (`self.Cube`) (`KismetMathLibrary.MakeRotator` (* X 10.0) (* Y 10.0)) false false))

(event `self.InteractionA`
  (params (Player :type "/Game/CHARACTER_AMETHYSTE/Blueprints/BP_CHARACTER Object Reference"))
  ;[1 1 1] verifie si on est deja entrain d'inspecter
  (if (not (`self.isInspecting`))
    (set `self.StartPoint` (`SceneComponent.K2_GetComponentToWorld` (`self.Cube`)))
    (set `self.EndPoint` (`SceneComponent.K2_GetComponentToWorld` (`/Game/CHARACTER_AMETHYSTE/Blueprints/BP_CHARACTER.Arrow1` Player)))
    (`PrimitiveComponent.SetEnableGravity` (`self.Cube`) false)
    (set `/Game/CHARACTER_AMETHYSTE/Blueprints/BP_CHARACTER.canMove` false Player)
    (set `/Game/CHARACTER_AMETHYSTE/Blueprints/BP_CHARACTER.canLook` false Player)
    (set `self.isInspecting` true)
    (set `/Game/CHARACTER_AMETHYSTE/Blueprints/BP_CHARACTER.IsGrabbingObject` true Player)
    (`PrimitiveComponent.SetCollisionEnabled` (`self.Cube`) "QueryOnly")
    (bind (_direction _delta) (`Timeline|zoom` :!label _label)
      (:`Update`
        (`SceneComponent.K2_SetWorldTransform` (`self.Cube`) (`KismetMathLibrary.MakeTransform` (.location (`KismetMathLibrary.TLerp` (`self.StartPoint`) (`self.EndPoint`) _delta)) (.rotation (`KismetMathLibrary.TLerp` (`self.StartPoint`) (`self.EndPoint`) _delta))) false false))
      (:`Finished`
        (if (not (`self.isInspecting`))
          (`PrimitiveComponent.SetCollisionEnabled` (`self.Cube`) "QueryAndPhysics")
          (`PrimitiveComponent.SetEnableGravity` (`self.Cube`) true))))
    (else
      (set `/Game/CHARACTER_AMETHYSTE/Blueprints/BP_CHARACTER.canMove` true Player)
      (set `/Game/CHARACTER_AMETHYSTE/Blueprints/BP_CHARACTER.canLook` true Player)
      (set `self.isInspecting` false)
      (set `/Game/CHARACTER_AMETHYSTE/Blueprints/BP_CHARACTER.IsGrabbingObject` false Player)
      (goto _label :!via `Reverse`))))

(event `self.InteractionB`
  (params (Player :type "/Game/CHARACTER_AMETHYSTE/Blueprints/BP_CHARACTER Object Reference"))
  (bind _physicshandle (`/Game/CHARACTER_AMETHYSTE/Blueprints/BP_CHARACTER.PhysicsHandle` Player))
  (bind _returnvalue (`self.GetComponentByClass` (`/Game/CHARACTER_AMETHYSTE/Blueprints/BP_CHARACTER.InteractibleObject` Player) "/Script/Engine.PrimitiveComponent"))
  ;[0.02604 0.02604 0.02604] Grab Object
  (`/Engine/EditorBlueprintResources/StandardMacros.FlipFlop`
    (:`A`
      (set `/Game/CHARACTER_AMETHYSTE/Blueprints/BP_CHARACTER.IsGrabbingObject` true Player)
      (`PhysicsHandleComponent.GrabComponentAtLocationWithRotation` :`self` _physicshandle :`Component` _returnvalue :`Location` (`SceneComponent.K2_GetComponentLocation` _returnvalue)))
    (:`B`
      (if (`/Game/CHARACTER_AMETHYSTE/Blueprints/BP_CHARACTER.IsGrabbingObject` Player)
        (`PhysicsHandleComponent.ReleaseComponent` _physicshandle)
        (set `/Game/CHARACTER_AMETHYSTE/Blueprints/BP_CHARACTER.IsGrabbingObject` false Player)))))

(fn `UserConstructionScript`
  (`parent.UserConstructionScript`))