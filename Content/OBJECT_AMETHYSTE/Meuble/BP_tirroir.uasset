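; BP_tirroir is an interactable furniture drawer that slides open and closed.
; Each InteractionC event flips a FlipFlop that alternately plays and reverses the Opening timeline.
; The timeline lerps the Tr component's relative location from StartPos to an X offset set by Deplacement, without sweep.
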(event `self.InteractionC`
  (params (Player :type "/Game/CHARACTER_AMETHYSTE/Blueprints/BP_CHARACTER Object Reference"))
  (bind _startpos (`self.startPos`))
  (`/Engine/EditorBlueprintResources/StandardMacros.FlipFlop`
    (:`A`
      (bind (_direction _delta) (`Timeline|opening` :!label _label)
        (:`Update`
          (`SceneComponent.K2_SetRelativeLocation` (`self.tr`) (`KismetMathLibrary.VLerp` _startpos (+ _startpos (`KismetMathLibrary.MakeVector` (`self.deplacement`))) _delta) false false))))
    (:`B`
      (goto _label :!via `Reverse`))))

(fn `UserConstructionScript`
  (`parent.UserConstructionScript`))