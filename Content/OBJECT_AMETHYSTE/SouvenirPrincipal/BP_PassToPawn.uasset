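; Trigger actor that hands player control from BP_CHARACTER to a freshly spawned BP_BANQUECHARA pawn.
; When BP_CHARACTER overlaps the Box, it spawns the pawn at the box's location and rotation and possesses it with player controller 0.
; It then adds an Enhanced Input mapping context, passes the pawn to the BM reference and calls SplineToCast on it.
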(event `self.Box.OnComponentBeginOverlap`
  (params (OverlappedComponent :type "PrimitiveComponent Object Reference") (OtherActor :type "Actor Object Reference") (OtherComp :type "PrimitiveComponent Object Reference") (OtherBodyIndex :type Integer) (bFromSweep :type Boolean) (SweepResult :type "HitResult Structure (by ref)"))
  (bind _box (`self.Box`))
  (bind _bm (`self.BM`))
  (if (== (`GameplayStatics.GetObjectClass` OtherActor) "/Game/CHARACTER_AMETHYSTE/Blueprints/BP_CHARACTER.BP_CHARACTER_C")
    (bind _returnvalue (`|SpawnActorFromClass` "/Game/CHARACTER_AMETHYSTE/Blueprints/BP_BANQUECHARA.BP_BANQUECHARA_C" (`KismetMathLibrary.MakeTransform` (`SceneComponent.K2_GetComponentLocation` _box) (`SceneComponent.K2_GetComponentRotation` _box)) "Undefined" "MultiplyWithRoot" null null))
    (`/Engine/EditorBlueprintResources/StandardMacros.IsValid` _returnvalue
      (:`Is Valid`
        (`Controller.Possess` (`GameplayStatics.GetPlayerController` 0) _returnvalue)
        (bind _asplayer_controller (cast `PlayerController` (`GameplayStatics.GetPlayerController` 0)))
        (bind _returnvalue_2 (pcsubsystem `EnhancedInputLocalPlayerSubsystem` _asplayer_controller))
        (`/Engine/EditorBlueprintResources/StandardMacros.IsValid` _returnvalue_2
          (:`Is Valid`
            (`EnhancedInputSubsystemInterface.AddMappingContext` _returnvalue_2 null 1 (struct))
            (set `/Game/OBJECT_AMETHYSTE/SouvenirPrincipal/BP_BanqueManager.pawn` _returnvalue _bm)
            (`/Game/OBJECT_AMETHYSTE/SouvenirPrincipal/BP_BanqueManager.SplineToCast` _bm)))))))

(fn `UserConstructionScript`)