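; BP_EnterBanque is a trigger volume, apparently for entering the bank, that changes how far the player character's raycast reaches.
; When a BP_CHARACTER begins overlapping the Box, it greatly extends that character's RaycastLength.
; When the character ends the overlap, it sets RaycastLength to a fixed short range rather than restoring a saved value.
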(event `self.Box.OnComponentBeginOverlap`
  (params (OverlappedComponent :type "PrimitiveComponent Object Reference") (OtherActor :type "Actor Object Reference") (OtherComp :type "PrimitiveComponent Object Reference") (OtherBodyIndex :type Integer) (bFromSweep :type Boolean) (SweepResult :type "HitResult Structure (by ref)"))
  (if (== (`GameplayStatics.GetObjectClass` OtherActor) "/Game/CHARACTER_AMETHYSTE/Blueprints/BP_CHARACTER.BP_CHARACTER_C")
    (bind _asbp_character (cast `/Game/CHARACTER_AMETHYSTE/Blueprints/BP_CHARACTER` OtherActor))
    (set `/Game/CHARACTER_AMETHYSTE/Blueprints/BP_CHARACTER.RaycastLength` 10000.0 _asbp_character)))

(event `self.Box.OnComponentEndOverlap`
  (params (OverlappedComponent :type "PrimitiveComponent Object Reference") (OtherActor :type "Actor Object Reference") (OtherComp :type "PrimitiveComponent Object Reference") (OtherBodyIndex :type Integer))
  (if (== (`GameplayStatics.GetObjectClass` OtherActor) "/Game/CHARACTER_AMETHYSTE/Blueprints/BP_CHARACTER.BP_CHARACTER_C")
    (bind _asbp_character (cast `/Game/CHARACTER_AMETHYSTE/Blueprints/BP_CHARACTER` OtherActor))
    (set `/Game/CHARACTER_AMETHYSTE/Blueprints/BP_CHARACTER.RaycastLength` 200.0 _asbp_character)))

(fn `UserConstructionScript`)